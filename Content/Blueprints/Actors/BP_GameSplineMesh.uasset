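; Spline mesh actor that visualizes progress along a line, apparently the player's, using the M_PlayerOnLine material.
; BeginPlay creates a dynamic material instance and applies it to the spline mesh.
; Each Tick pushes LineProgress and two blue colors into it; when IsReverse is false, the progress is inverted and the light and dark colors are swapped.
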(event EventBeginPlay
  (bind _splinemeshcomponent (Variables|Default|GetSplineMeshComponent))
  (bind _returnvalue (Rendering|Material|CreateDynamicMaterialInstance _splinemeshcomponent 0 "/Game/Materials/M_PlayerOnLine.M_PlayerOnLine" "None" :!class /Script/Engine.PrimitiveComponent))
  (bind _output_get (Variables|Default|SetDynamicMaterial _returnvalue))
  (Rendering|Material|SetMaterial _splinemeshcomponent 0 _output_get))

(event Collision|EventActorBeginOverlap
  (params (OtherActor :type Actor%20Object%20Reference)))

(event EventTick
  (params (DeltaSeconds :type Float%20%28single-precision%29))
  (bind _dynamicmaterial (Variables|Default|GetDynamicMaterial))
  (bind _dynamicmaterial_2 (Variables|Default|GetDynamicMaterial))
  (if (Variables|Default|GetbIsReverse)
    (Rendering|Material|SetScalarParameterValue _dynamicmaterial "LineProgress" (Variables|Default|GetLineProgress) :!class /Script/Engine.MaterialInstanceDynamic)
    (Rendering|Material|SetVectorParameterValue _dynamicmaterial "Blue" (Math|Conversions|ToLinearColor(Vector) "0.200000,0.200000,1.000000") :!class /Script/Engine.MaterialInstanceDynamic)
    (Rendering|Material|SetVectorParameterValue _dynamicmaterial "DarkBlue" (Math|Conversions|ToLinearColor(Vector) "0, 0,0.100000") :!class /Script/Engine.MaterialInstanceDynamic)
    (else
      (Rendering|Material|SetScalarParameterValue _dynamicmaterial_2 "LineProgress" (- 1.0 (Variables|Default|GetLineProgress)) :!class /Script/Engine.MaterialInstanceDynamic)
      (Rendering|Material|SetVectorParameterValue _dynamicmaterial_2 "Blue" (Math|Conversions|ToLinearColor(Vector) "0, 0,0.100000") :!class /Script/Engine.MaterialInstanceDynamic)
      (Rendering|Material|SetVectorParameterValue _dynamicmaterial_2 "DarkBlue" (Math|Conversions|ToLinearColor(Vector) "0.200000,0.200000,1.000000") :!class /Script/Engine.MaterialInstanceDynamic))))

(fn ConstructionScript)