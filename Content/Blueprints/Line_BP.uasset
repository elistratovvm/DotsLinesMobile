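; Line_BP is an actor that draws straight-line connectors between dots, linking Dot0 to Dot1 and Dot1 to Dot2 on BeginPlay.
; CreateSpline spawns a GameSplineMesh actor at the first dot, offsets its end to the second, and skins it with a scaled Z-forward cylinder.
; An alternative CreateCable using zero-gravity CableActors and a Level_1_DotsInfo table lookup are present but never run.
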(event EventBeginPlay
  (CallFunction|CreateSpline (Variables|Default|GetDot_0) (Variables|Default|GetDot_1))
  (CallFunction|CreateSpline (Variables|Default|GetDot_1) (Variables|Default|GetDot_2)))

(event Collision|EventActorBeginOverlap
  (params (OtherActor :type Actor%20Object%20Reference)))

(event EventTick
  (params (DeltaSeconds :type Float%20%28single-precision%29)))

(fn ConstructionScript)

(fn CreateCable
  (params (Pos_1 :type Static%20Mesh%20Component%20Object%20Reference) (Pos_2 :type Static%20Mesh%20Component%20Object%20Reference))
  (bind _returnvalue (Game|SpawnActorfromClass "/Script/CableComponent.CableActor" (Transformation|GetWorldTransform Pos_1) "AlwaysSpawn" 0 0))
  (bind _output_get (Variables|Default|SetCable_01 _returnvalue))
  (Variables|/Script/CableComponent.CableComponent|SetCableGravityScale (Variables|/Script/CableComponent.CableActor|GetCableComponent _output_get) 0.0)
  (Variables|/Script/CableComponent.CableComponent|SetEndLocation (Variables|/Script/CableComponent.CableActor|GetCableComponent _output_get) "0, 0, 0")
  (Class|CableComponent|SetAttachEndtoComponent (Variables|/Script/CableComponent.CableActor|GetCableComponent _output_get) Pos_2 "None"))

(fn CreateSpline
  (params (Pos_1 :type Static%20Mesh%20Component%20Object%20Reference) (Pos_2 :type Static%20Mesh%20Component%20Object%20Reference))
  (bind _returnvalue (Game|SpawnActorfromClass "/Script/MobileGameElistratov.GameSplineMesh" (Transformation|GetWorldTransform Pos_1) "AlwaysSpawn" self 0))
  (bind _output_get (LocalVariables|SetThis_Spline_MC (Variables|/Script/MobileGameElistratov.GameSplineMesh|GetSplineMeshComponent _returnvalue)))
  (SplineMesh|SetEndPosition _output_get (- (Transformation|GetWorldLocation Pos_2) (Transformation|GetWorldLocation (Variables|/Script/MobileGameElistratov.GameSplineMesh|GetSplineMeshComponent _returnvalue))) true)
  (Components|StaticMesh|SetStaticMesh (LocalVariables|GetThis_Spline_MC) "/Engine/BasicShapes/Cylinder.Cylinder")
  (SplineMesh|SetForwardAxis (LocalVariables|GetThis_Spline_MC) "Z" true)
  (SplineMesh|SetStartScale (LocalVariables|GetThis_Spline_MC) "(X=0.800000,Y=0.800000)" true :!class /Script/Engine.SplineMeshComponent)
  (SplineMesh|SetEndScale (LocalVariables|GetThis_Spline_MC) "(X=0.800000,Y=0.800000)" true :!class /Script/Engine.SplineMeshComponent))