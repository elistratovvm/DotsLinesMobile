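; GameManager_BP is a game manager actor that sets up the player's view and opens the main menu.
; On BeginPlay, SetUpCamera makes the actor itself player 0's view target, then a main menu widget is created and added to the viewport.
; Leftover DrawLines calls and mouse and HUD lookups are unconnected and never run.
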(event EventBeginPlay
  (CallFunction|SetUpCamera)
  (bind _returnvalue (UserInterface|CreateWidget "/Game/Widgets/WDBP_MainMenu.WDBP_MainMenu_C"))
  (UserInterface|Viewport|AddtoViewport _returnvalue 0))

(event Collision|EventActorBeginOverlap
  (params (OtherActor :type Actor%20Object%20Reference)))

(event EventTick
  (params (DeltaSeconds :type Float%20%28single-precision%29)))

(event Input|TouchEvents|Touch1
  (params (Key :type Key%20Structure :default "None")))

(fn ConstructionScript)

(fn SetUpCamera
  (Game|Player|SetViewTargetwithBlend (Game|GetPlayerController 0) self 0.0 "VTBlend_Linear" 0.0 false))